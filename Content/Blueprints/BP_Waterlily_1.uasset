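; BP_Waterlily_1 is a collectible water lily sample that the player picks up for research.
; Pressing E traces 500 units forward from the camera, prints the hit actor's name and destroys it if its class name matches the lily's.
; It then counts the remaining lilies and, at exactly 18, reports two more samples are needed.
; The other progress messages, including completion, sit in disconnected branches that never run.
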(event `self.ReceiveBeginPlay`)

(event `Key|E` :consume false
  (params (Key :type "Key Structure"))
  (bind _returnvalue (`GameplayStatics.GetPlayerCameraManager` 0))
  (bind _returnvalue_2 (`self.K2_GetActorLocation` _returnvalue))
  (:`Pressed`
    (bind _outhit (`KismetSystemLibrary.LineTraceSingleForObjects` :`Start` _returnvalue_2 :`End` (+ _returnvalue_2 (* (`self.GetActorForwardVector` _returnvalue) 500.0)) :`ObjectTypes` (`|MakeArray` "ObjectTypeQuery2" :!type "EObjectTypeQuery Enum") :`bIgnoreSelf` false))
    (bind (_bblockinghit _binitialoverlap _time _distance _location _impactpoint _normal _impactnormal _physmat _hitactor) (`GameplayStatics.BreakHitResult` _outhit))
    (`KismetSystemLibrary.PrintString` (`KismetSystemLibrary.GetDisplayName` _hitactor))
    (if (`KismetStringLibrary.EqualEqual_StrStr` (`KismetSystemLibrary.GetClassDisplayName` (`GameplayStatics.GetObjectClass` _hitactor)) (`KismetSystemLibrary.GetClassDisplayName` "BP_Waterlily_1_C"))
      (`self.K2_DestroyActor` _hitactor)
      (bind _outactors (`GameplayStatics.GetAllActorsOfClass` "BP_Waterlily_1_C"))
      (`/Engine/EditorBlueprintResources/StandardMacros.CompareInt` (`KismetArrayLibrary.Array_Length` _outactors) 18
        (:`==`
          (`KismetSystemLibrary.PrintString` "You found a water lily, but you need 2 more samples."))))))

(fn `UserConstructionScript`)